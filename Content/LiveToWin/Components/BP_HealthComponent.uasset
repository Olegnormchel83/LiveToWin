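; BP_HealthComponent is an actor component that tracks an owner's integer Health and MaxHealth.
; It fills Health to MaxHealth on BeginPlay, and its increase and decrease functions keep Health between zero and MaxHealth.
; Changes fire health-changed or max-health-changed dispatchers, and a decrease that reaches zero also fires the death dispatcher.
; Updating MaxHealth leaves current Health untouched.
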(event `self.ReceiveBeginPlay`
  (`self.RestoreHealth`))

(fn `DecreaseHealth`
  (params (Value :type Integer))
  (bind _returnvalue (- (`self.Health`) Value))
  (if (<= _returnvalue 0)
    (set `self.Health` 0)
    (`self.OnHealthChanged` (`self.Health`))
    (`self.OnDead`)
    (else
      (set `self.Health` (`KismetMathLibrary.Clamp` _returnvalue 0 (`self.MaxHealth`)))
      (`self.OnHealthChanged` (`self.Health`)))))

(fn `GetHealth`
  (returns (Health :type Integer))
  (return (`self.Health`)))

(fn `GetMaxHealth`
  (returns (MaxHealth :type Integer))
  (return (`self.MaxHealth`)))

(fn `IncreaseHealth`
  (params (Value :type Integer))
  (set `self.Health` (`KismetMathLibrary.Clamp` (+ (`self.Health`) Value) 0 (`self.MaxHealth`)))
  (`self.OnHealthChanged` (`self.Health`)))

(fn `RestoreHealth`
  (set `self.Health` (`self.MaxHealth`))
  (`self.OnHealthChanged` (`self.Health`)))

(fn `UpdateMaxHealth`
  (params (NewMaxHealth :type Integer))
  (set `self.MaxHealth` NewMaxHealth)
  (`self.OnMaxHealthChanged` (`self.MaxHealth`)))