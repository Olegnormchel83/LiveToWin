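; Actor component that holds a character's Power, Agility and Stamina attributes, randomized within a small range on BeginPlay.
; Add functions raise one stat, rebuild the Attributes struct and fire OnAttributesUpdated, passing the added amount rather than the new total for that stat.
; SetAttributesHandle overwrites all three without firing the event.
; Getters expose the values separately or as the struct.
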(event `self.ReceiveBeginPlay`
  (`self.InitAttributes`))

(fn `AddAgility`
  (params (Value :type Integer))
  (set `self.Agility` (+ (`self.Agility`) Value))
  (set `self.Attributes` (make `/Game/LiveToWin/Components/F_Attributes` (`self.Power`) (`self.Agility`) (`self.Stamina`)))
  (`self.OnAttributesUpdated` (`self.Power`) Value (`self.Stamina`)))

(fn `AddPower`
  (params (Value :type Integer))
  (set `self.Power` (+ (`self.Power`) Value))
  (set `self.Attributes` (make `/Game/LiveToWin/Components/F_Attributes` (`self.Power`) (`self.Agility`) (`self.Stamina`)))
  (`self.OnAttributesUpdated` Value (`self.Agility`) (`self.Stamina`)))

(fn `AddStamina`
  (params (Value :type Integer))
  (set `self.Stamina` (+ (`self.Stamina`) Value))
  (set `self.Attributes` (make `/Game/LiveToWin/Components/F_Attributes` (`self.Power`) (`self.Agility`) (`self.Stamina`)))
  (`self.OnAttributesUpdated` (`self.Power`) (`self.Agility`) Value))

(fn `GetAttributes`
  (returns (Power :type Integer) (Agility :type Integer) (Stamina :type Integer))
  (return (`self.Power`) (`self.Agility`) (`self.Stamina`)))

(fn `GetAttributesStruct`
  (returns (Attributes :type "/Game/LiveToWin/Components/F_Attributes Structure"))
  (return (`self.Attributes`)))

(fn `InitAttributes`
  (bind _returnvalue (`KismetMathLibrary.RandomIntegerInRange` 1 3))
  (set `self.Power` _returnvalue)
  (set `self.Agility` _returnvalue)
  (set `self.Stamina` _returnvalue)
  (set `self.Attributes` (make `/Game/LiveToWin/Components/F_Attributes` (`self.Power`) (`self.Agility`) (`self.Stamina`)))
  (`self.OnAttributesUpdated` (`self.Power`) (`self.Agility`) (`self.Stamina`)))

(fn `SetAttributesHandle`
  (params (Power :type Integer) (Agility :type Integer) (Stamina :type Integer))
  (set `self.Power` Power)
  (set `self.Agility` Agility)
  (set `self.Stamina` Stamina)
  (set `self.Attributes` (make `/Game/LiveToWin/Components/F_Attributes` (`self.Power`) (`self.Agility`) (`self.Stamina`))))