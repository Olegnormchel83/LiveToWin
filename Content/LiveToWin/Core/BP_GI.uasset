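; BP_GI is the Blueprint for LiveToWin's game instance, which sets default graphics settings at startup.
; On Init it gets Game User Settings, caps the frame rate at 60 and sets each scalability category to a hard-coded, mostly low quality level.
; The graph only calls setters and never applies or saves the settings.
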(event `self.ReceiveInit`
  (bind _returnvalue (`GameUserSettings.GetGameUserSettings`))
  (`GameUserSettings.SetFrameRateLimit` _returnvalue 60.0)
  (`GameUserSettings.SetViewDistanceQuality` _returnvalue 0)
  (`GameUserSettings.SetAntiAliasingQuality` _returnvalue 0)
  (`GameUserSettings.SetPostProcessingQuality` _returnvalue 2)
  (`GameUserSettings.SetShadowQuality` _returnvalue 1)
  (`GameUserSettings.SetGlobalIlluminationQuality` _returnvalue 0)
  (`GameUserSettings.SetReflectionQuality` _returnvalue 0)
  (`GameUserSettings.SetTextureQuality` _returnvalue 1)
  (`GameUserSettings.SetVisualEffectQuality` _returnvalue 1)
  (`GameUserSettings.SetShadingQuality` _returnvalue 1))