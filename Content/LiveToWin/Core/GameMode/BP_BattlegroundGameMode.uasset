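; Battleground game mode that runs an automatic turn-based duel between one player character and one enemy.
; On BeginPlay it switches the view to the level's camera actor, finds both combatants and binds their attack-ended events.
; Higher Stamina attacks first, with ties going to the player.
; Each attack-ended event passes the turn to the other side through a timer delay, printing debug messages in Russian.
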(event `self.ReceiveBeginPlay`
  (bind _returnvalue (`GameplayStatics.GetActorOfClass` "/Game/LiveToWin/Core/BP_CameraActor.BP_CameraActor_C"))
  (`PlayerController.SetViewTargetWithBlend` (`GameplayStatics.GetPlayerController` 0) _returnvalue 0.0 "VTBlend_Linear" 0.0 false)
  (bind _returnvalue_2 (`GameplayStatics.GetActorOfClass` "/Game/LiveToWin/Core/Characters/BP_BaseCharacter.BP_BaseCharacter_C"))
  (bind _output_get (set `self.PlayerCharacter` _returnvalue_2))
  (add `/Game/LiveToWin/Core/Characters/BP_BaseCharacter.OnPlayerAttackEnded` _output_get (delegate `OnPlayerAttackEnded_Event`))
  (bind _returnvalue_3 (`GameplayStatics.GetActorOfClass` "/Game/LiveToWin/Core/Characters/BP_BaseEnemy.BP_BaseEnemy_C"))
  (bind _output_get_2 (set `self.EnemyCharacter` _returnvalue_3))
  (add `/Game/LiveToWin/Core/Characters/BP_BaseEnemy.OnEnemyAttackEnded` _output_get_2 (delegate `OnEnemyAttackEnded_Event`))
  (bind _value (`self.CompareCharactersForFirstAttack`))
  (set `self.Value` _value)
  (`self.CharacterAttack`))

(event `OnPlayerAttackEnded_Event`
  (`KismetSystemLibrary.PrintString` "Игрок закончил атаку")
  (set `self.Value` 0)
  (`self.CharacterAttack`))

(event `OnEnemyAttackEnded_Event`
  (`KismetSystemLibrary.PrintString` "Противник закончил атаку")
  (set `self.Value` 1)
  (`self.CharacterAttack`))

(event `CharacterAttack`
  (`KismetSystemLibrary.K2_SetTimerDelegate` (delegate `Attack`) (`self.TimeBetweenAttacks`)))

(event `Attack`
  (if (== (`self.Value`) 0)
    (`KismetSystemLibrary.PrintString` "Противник начал атаку")
    (`/Game/LiveToWin/Core/Characters/BP_BaseEnemy.Attack` (`self.EnemyCharacter`))
    (else
      (`KismetSystemLibrary.PrintString` "Игрок начал атаку")
      (`/Game/LiveToWin/Core/Characters/BP_BaseCharacter.Attack` (`self.PlayerCharacter`)))))

(fn `CompareCharactersForFirstAttack`
  (returns (Value :type Integer))
  (bind _playercharacter (`self.PlayerCharacter`)
    (:`then`
      (bind _enemycharacter (`self.EnemyCharacter`)
        (:`then`
          (return (select `bool` (> (`.Stamina` (`/Game/LiveToWin/Components/BP_AttributesComponent.GetAttributes` (`/Game/LiveToWin/Core/Characters/BP_BaseEnemy.BP_AttributesComponent` _enemycharacter))) (`.Stamina` (`/Game/LiveToWin/Components/BP_AttributesComponent.GetAttributes` (`/Game/LiveToWin/Core/Characters/BP_BaseCharacter.BP_AttributesComponent` _playercharacter)))) :`false` 1)))
        (:`else`)))
    (:`else`)))

(fn `UserConstructionScript`)