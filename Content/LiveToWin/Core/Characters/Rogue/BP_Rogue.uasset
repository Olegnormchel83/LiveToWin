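; BP_Rogue is the Rogue character class, a child Blueprint that layers class-specific health bonuses onto its parent.
; On BeginPlay it adds the first specialization enum value, then raises max health by the Stamina attribute before calling the parent.
; Its AddSpecialization override grants a flat max health bonus through the health component before passing the specialization to the parent.
; A debug print about level-up health is left disconnected.
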(event `self.ReceiveBeginPlay`
  (bind _bp_healthcomponent (`self.BP_HealthComponent`))
  (`self.AddSpecialization` "NewEnumerator0")
  (`/Game/LiveToWin/Components/BP_HealthComponent.UpdateMaxHealth` _bp_healthcomponent (+ (`/Game/LiveToWin/Components/BP_HealthComponent.GetMaxHealth` _bp_healthcomponent) (`.Stamina` (`/Game/LiveToWin/Components/BP_AttributesComponent.GetAttributes` (`self.BP_AttributesComponent`)))))
  (`parent.ReceiveBeginPlay`))

(fn `AddSpecialization`
  (params (Spec :type "/Game/LiveToWin/Core/Characters/E_CharacterClass Enum" :default "NewEnumerator3"))
  (bind _bp_healthcomponent (`self.BP_HealthComponent`))
  (`/Game/LiveToWin/Components/BP_HealthComponent.UpdateMaxHealth` _bp_healthcomponent (+ (`/Game/LiveToWin/Components/BP_HealthComponent.GetMaxHealth` _bp_healthcomponent) 4))
  (`parent.AddSpecialization` Spec))

(fn `UserConstructionScript`
  (`parent.UserConstructionScript`))