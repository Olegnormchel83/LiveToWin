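; Base combat character that spawns a socketed weapon, derives max health and weapon damage from attributes, and tracks leveled specializations.
; Attack traces for an enemy, runs up until within range, plays a random montage with delayed weapon collision, then returns to its start position and signals attack end.
; Timers poll range and arrival.
; Incoming damage shows an animated number, zeroed by an agility-based hit check.
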(event `self.ReceiveEndPlay`
  (params (EndPlayReason :type "EEndPlayReason Enum" :default "Destroyed"))
  (bind _bp_attributescomponent (`self.BP_AttributesComponent`)
    (:`then`
      (clear `/Game/LiveToWin/Components/BP_AttributesComponent.OnAttributesUpdated` _bp_attributescomponent)
      (bind _bp_healthcomponent (`self.BP_HealthComponent`)
        (:`then`
          (clear `/Game/LiveToWin/Components/BP_HealthComponent.OnHealthChanged` _bp_healthcomponent)
          (clear `/Game/LiveToWin/Components/BP_HealthComponent.OnDead` _bp_healthcomponent))
        (:`else`)))
    (:`else`)))

(event `self.ReceiveBeginPlay`
  (bind _bp_healthcomponent (`self.BP_HealthComponent`))
  (bind (_power _agility _stamina) (`/Game/LiveToWin/Components/BP_AttributesComponent.GetAttributes` (`self.BP_AttributesComponent`)))
  (bind _bp_attributescomponent (`self.BP_AttributesComponent`)
    (:`then`
      (add `/Game/LiveToWin/Components/BP_AttributesComponent.OnAttributesUpdated` _bp_attributescomponent (`|CreateDelegate` :!event `InAttributesUpdated_Event`))
      (bind _bp_healthcomponent_2 (`self.BP_HealthComponent`)
        (:`then`
          (add `/Game/LiveToWin/Components/BP_HealthComponent.OnHealthChanged` _bp_healthcomponent_2 (`|CreateDelegate` :!event `OnHealthChanged_Event`))
          (add `/Game/LiveToWin/Components/BP_HealthComponent.OnDead` _bp_healthcomponent_2 (`|CreateDelegate` :!event `OnDead_Event`))
          (bind _returnvalue (`|SpawnActorFromClass` (`self.WeaponClass`) (`KismetMathLibrary.MakeTransform` (0.0 0.0 0.0)) "AlwaysSpawn" "MultiplyWithRoot" self null))
          (`/Engine/EditorBlueprintResources/StandardMacros.IsValid` _returnvalue
            (:`Is Valid`
              (bind _output_get (set `self.Weapon` _returnvalue))
              (`self.K2_AttachToComponent` _output_get (`self.Mesh`) "WeaponSocket" "SnapToTarget" "SnapToTarget" "SnapToTarget" true))
            (:`Is Not Valid`
              (`KismetSystemLibrary.PrintString` (`KismetStringLibrary.Concat_StrStr` "Warning: " "Unsuccessfull spawning weapon (Weapon nullptr)"))))
          (`/Game/LiveToWin/Components/BP_HealthComponent.UpdateMaxHealth` _bp_healthcomponent (+ (`/Game/LiveToWin/Components/BP_HealthComponent.GetMaxHealth` _bp_healthcomponent) _stamina))
          (`/Game/LiveToWin/Components/BP_HealthComponent.RestoreHealth` _bp_healthcomponent)
          (`/Game/LiveToWin/Weapons/BP_WeaponBase.AddDamageByPower` (`self.Weapon`) _power)
          (set `self.StartPosition` (`self.K2_GetActorLocation`)))
        (:`else`)))
    (:`else`)))

(event `OnHealthChanged_Event`
  (params (NewHealth :type Integer)))

(event `OnDead_Event`)

(event `InAttributesUpdated_Event`
  (params (UpdatedPower :type Integer) (UpdatedAgility :type Integer) (UpdatedStamina :type Integer))
  (bind _bp_healthcomponent (`self.BP_HealthComponent`))
  (`/Game/LiveToWin/Components/BP_HealthComponent.UpdateMaxHealth` _bp_healthcomponent (+ (`/Game/LiveToWin/Components/BP_HealthComponent.GetMaxHealth` _bp_healthcomponent) UpdatedStamina))
  (`/Game/LiveToWin/Components/BP_HealthComponent.RestoreHealth` _bp_healthcomponent))

(event `self.ReceiveAnyDamage`
  (params (Damage :type "Float (single-precision)") (DamageType :type "DamageType Object Reference") (InstigatedBy :type "Controller Object Reference") (DamageCauser :type "Actor Object Reference"))
  (bind _returnvalue (`WidgetComponent.GetWidget` (`self.Widget`)))
  (bind _attagility (message `/Game/LiveToWin/Interfaces/BPI_Battlable.GetAgility` DamageCauser))
  (bind _attagility_2 (`self.GetAgility`))
  (bind _miss (`/Game/LiveToWin/BFL_Battle.CalculateHitRate` _attagility _attagility_2))
  (if _miss
    (message `/Game/LiveToWin/Interfaces/BPI_WDamageValue.SetDamageValue` _returnvalue 0)
    (else
      (message `/Game/LiveToWin/Interfaces/BPI_WDamageValue.SetDamageValue` _returnvalue (`KismetMathLibrary.FTrunc` Damage))))
  (`Widget.SetVisibility` _returnvalue "SelfHitTestInvisible")
  (bind _newparam (message `/Game/LiveToWin/Interfaces/BPI_WDamageValue.GetAnimation` _returnvalue))
  (`|PlayAnimation` _returnvalue _newparam 0.0 1 "Forward" 0.3
    (:`Finished`
      (`Widget.SetVisibility` _returnvalue "Collapsed"))))

(fn `AddSpecialization`
  (params (Spec :type "/Game/LiveToWin/Core/Characters/E_CharacterClass Enum" :default "NewEnumerator0"))
  (`KismetArrayLibrary.Array_AddUnique` (`self.Specialization`) (make `/Game/LiveToWin/Core/Characters/F_Specialization` Spec)))

(fn `Attack`
  (bind _returnvalue (`self.K2_GetActorLocation`))
  (bind _outhit (`KismetSystemLibrary.LineTraceSingle` :`Start` _returnvalue :`End` (+ _returnvalue (* (`self.GetActorForwardVector`) 3000.0)) :`TraceChannel` "TraceTypeQuery3" :`DrawDebugType` "ForDuration"))
  (bind (_bblockinghit _binitialoverlap _time _distance _location _impactpoint _normal _impactnormal _physmat _hitactor) (`GameplayStatics.BreakHitResult` _outhit))
  (if (`GameplayStatics.ObjectIsA` _hitactor "/Game/LiveToWin/Core/Characters/BP_BaseEnemy.BP_BaseEnemy_C")
    (bind _output_get (set `self.EnemyPosition` (`self.K2_GetActorLocation` _hitactor)))
    (`AIBlueprintHelperLibrary.SimpleMoveToLocation` (`self.GetController`) _output_get)
    (bind _returnvalue_2 (`KismetSystemLibrary.K2_SetTimer` null "FindEnemy" 0.1 true))
    (set `self.FindEnemyTimerHandle` _returnvalue_2)))

(fn `EnableWeaponCollision`
  (`PrimitiveComponent.SetCollisionEnabled` (`/Game/LiveToWin/Weapons/BP_WeaponBase.DetectCapsule` (`self.Weapon`)) "QueryOnly"))

(fn `FindEnemy`
  (bind _returnvalue (`self.K2_GetActorLocation`))
  (bind _outhit (`KismetSystemLibrary.LineTraceSingle` :`Start` _returnvalue :`End` (+ _returnvalue (* (`self.GetActorForwardVector`) (`self.AttackRange`))) :`TraceChannel` "TraceTypeQuery3" :`DrawDebugType` "ForOneFrame"))
  (if (`GameplayStatics.ObjectIsA` (`.HitActor` (`GameplayStatics.BreakHitResult` _outhit)) "/Game/LiveToWin/Core/Characters/BP_BaseEnemy.BP_BaseEnemy_C")
    (`KismetSystemLibrary.K2_ClearAndInvalidateTimerHandle` (`self.FindEnemyTimerHandle`))
    (`MovementComponent.StopMovementImmediately` (`self.CharacterMovement`))
    (`self.MakeHit`)))

(fn `GetAgility`
  (returns (AttAgility :type Integer))
  (return (`/Game/LiveToWin/Components/BP_AttributesComponent.Agility` (`self.BP_AttributesComponent`))))

(fn `GetAttributesStruct`
  (returns (Attributes :type "/Game/LiveToWin/Components/F_Attributes Structure"))
  (return (`/Game/LiveToWin/Components/BP_AttributesComponent.GetAttributesStruct` (`self.BP_AttributesComponent`))))

(fn `GetWeapon`
  (returns (Weapon :type "/Game/LiveToWin/Weapons/BP_WeaponBase Object Reference"))
  (return (`self.Weapon`)))

(fn `GetWeaponInfo`
  (returns (WeaponInfo :type "/Game/LiveToWin/Weapons/F_WeaponInfo Structure"))
  (return (`/Game/LiveToWin/Weapons/BP_WeaponBase.WeaponInfo` (`self.Weapon`))))

(fn `IsAtStartLocation`
  (bind (_returnvalue_x _returnvalue_y) (`KismetMathLibrary.BreakVector` (`self.K2_GetActorLocation`)))
  (bind (_startposition_x _startposition_y) (`KismetMathLibrary.BreakVector` (`self.StartPosition`)))
  (if (and (`KismetMathLibrary.NearlyEqual_FloatFloat` _returnvalue_x _startposition_x 1.0) (`KismetMathLibrary.NearlyEqual_FloatFloat` _returnvalue_y _startposition_y 1.0))
    (`self.K2_SetActorRotation` (`KismetMathLibrary.FindLookAtRotation` (`self.K2_GetActorLocation`) (`self.EnemyPosition`)))
    (`KismetSystemLibrary.K2_ClearAndInvalidateTimerHandle` (`self.CheckStartLocationTimerHandle`))
    (`self.OnPlayerAttackEnded`)))

(fn `IsAttacking`
  (returns (Attacking :type Boolean))
  (return (`self.bAttacking`)))

(fn `MakeHit`
  (bind _attackanims (`self.AttackAnims`))
  (if (`KismetArrayLibrary.Array_IsNotEmpty` _attackanims)
    (bind _returnvalue (`self.PlayAnimMontage` (`KismetArrayLibrary.Array_Random` _attackanims)))
    (set `self.bAttacking` true)
    (`KismetSystemLibrary.K2_SetTimer` null "ReturnOnStartPosition" _returnvalue)
    (`KismetSystemLibrary.K2_SetTimer` null "EnableWeaponCollision" (* _returnvalue 0.35))))

(fn `ReturnOnStartPosition`
  (bind _startposition (`self.StartPosition`))
  (set `self.bAttacking` false)
  (`self.K2_SetActorRotation` (`KismetMathLibrary.FindLookAtRotation` (`self.K2_GetActorLocation`) _startposition))
  (`AIController.MoveToLocation` (`AIBlueprintHelperLibrary.GetAIController` self) _startposition 1.0 false true false true null true)
  (bind _returnvalue (`KismetSystemLibrary.K2_SetTimer` null "IsAtStartLocation" 0.1 true))
  (set `self.CheckStartLocationTimerHandle` _returnvalue))

(fn `SpecializationUp`
  (params (Spec :type "/Game/LiveToWin/Core/Characters/E_CharacterClass Enum" :default "NewEnumerator0"))
  (for (_array_element _array_index) (`self.Specialization`)
    (bind (_specialization _level) (break `/Game/LiveToWin/Core/Characters/F_Specialization` _array_element))
    (if (`|EnumEquality` _specialization Spec)
      (`KismetArrayLibrary.Array_Set` (`self.Specialization`) _array_index (make `/Game/LiveToWin/Core/Characters/F_Specialization` _specialization (+ _level 1))))))

(fn `UserConstructionScript`)