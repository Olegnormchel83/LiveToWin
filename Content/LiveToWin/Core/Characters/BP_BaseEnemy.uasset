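; Base enemy character that spawns its typed weapon, applies stats and shows an info widget.
; Attack line-traces for the player, advances until in range, plays a random montage with delayed weapon collision, then returns to its start position and signals attack end, sequenced by timers.
; Damage or misses show an animated message.
; Death ragdolls the body, then fires EnemyDied after a delay; CalculateFinalDamage is a zero-returning stub.
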(event `self.ReceiveBeginPlay`
  (bind (_damage _damagetype) (`/Game/LiveToWin/Weapons/BP_WeaponBase.GetWeaponInfo` (`self.Weapon`)))
  (bind (_power _agility _stamina) (`/Game/LiveToWin/Components/BP_AttributesComponent.GetAttributes` (`self.BP_AttributesComponent`)))
  (bind _bp_attributescomponent (`self.BP_AttributesComponent`)
    (:`then`
      (`/Game/LiveToWin/Components/BP_AttributesComponent.SetAttributesHandle` _bp_attributescomponent (`self.Power`) (`self.Agility`) (`self.Stamina`))
      (bind _spawnedweapon (`self.SpawnWeapon` (select `/Game/LiveToWin/Weapons/E_Weapon` (`self.WeaponType`) :`NewEnumerator0` "/Game/LiveToWin/Weapons/Sword/BP_Sword.BP_Sword_C" :`NewEnumerator1` "/Game/LiveToWin/Weapons/Club/BP_Club.BP_Club_C" :`NewEnumerator2` "/Game/LiveToWin/Weapons/Dagger/BP_Dagger.BP_Dagger_C" :`NewEnumerator3` "/Game/LiveToWin/Weapons/Axe/BP_Axe.BP_Axe_C" :`NewEnumerator4` "/Game/LiveToWin/Weapons/Spear/BP_Spear.BP_Spear_C" :`NewEnumerator5` "/Game/LiveToWin/Weapons/LegendarySword/BP_LegendarySword.BP_LegendarySword_C" :!type "/Game/LiveToWin/Weapons/BP_WeaponBase Class Reference")))
      (bind _output_get (set `self.Weapon` _spawnedweapon))
      (`self.K2_AttachToComponent` _output_get (`self.Mesh`) "WeaponSocket" "SnapToTarget" "SnapToTarget" "SnapToTarget" true)
      (`/Game/LiveToWin/Weapons/BP_WeaponBase.SetDamage` _output_get (`self.WeaponDamage`))
      (bind _bp_healthcomponent (`self.BP_HealthComponent`)
        (:`then`
          (`/Game/LiveToWin/Components/BP_HealthComponent.UpdateMaxHealth` _bp_healthcomponent (`self.Health`))
          (`/Game/LiveToWin/Components/BP_HealthComponent.RestoreHealth` _bp_healthcomponent)
          (set `self.StartLocation` (`self.K2_GetActorLocation`))
          (add `/Game/LiveToWin/Components/BP_HealthComponent.OnHealthChanged` _bp_healthcomponent (delegate `OnHealthChanged_event`))
          (add `/Game/LiveToWin/Components/BP_HealthComponent.OnDead` _bp_healthcomponent (delegate `OnDead_Event`))
          (bind _returnvalue (`|CreateWidget` "/Game/LiveToWin/UI/Game/WBP_EnemyInfo.WBP_EnemyInfo_C" null (`self.Name`) (`/Game/LiveToWin/Components/BP_HealthComponent.GetHealth` (`self.BP_HealthComponent`)) _power _agility _stamina (`self.Bonus`) (`self.WeaponType`) _damage _damagetype))
          (bind _output_get_2 (set `self.InfoWidget` _returnvalue))
          (`UserWidget.AddToViewport` _output_get_2 0))
        (:`else`)))
    (:`else`)))

(event `OnDead_Event`
  (bind _mesh (`self.Mesh`))
  (`KismetSystemLibrary.K2_SetTimerDelegate` (delegate `EnemyDead`) 2.0)
  (`PrimitiveComponent.SetCollisionEnabled` (`self.Mesh`) "NoCollision")
  (`PrimitiveComponent.SetCollisionEnabled` (`self.CapsuleComponent`) "NoCollision")
  (`PrimitiveComponent.SetSimulatePhysics` _mesh true)
  (`PrimitiveComponent.SetCollisionProfileName` _mesh "Ragdoll" true))

(event `OnHealthChanged_event`
  (params (NewHealth :type Integer))
  (bind _infowidget (`self.InfoWidget`)
    (:`then`
      (`/Game/LiveToWin/UI/Game/WBP_EnemyInfo.UpdateHealth` _infowidget NewHealth))
    (:`else`)))

(event `EnemyDead`
  (`self.OnEnemyDied`)
  (bind _infowidget (`self.InfoWidget`)
    (:`then`
      (`Widget.RemoveFromParent` _infowidget)
      (set `self.InfoWidget` null))
    (:`else`)))

(event `OnAttackerMissed`
  (bind _returnvalue (`WidgetComponent.GetWidget` (`self.Widget_Damage`)))
  (message `/Game/LiveToWin/Interfaces/BPI_WDamageValue.SetDamageValue` _returnvalue 0 :!label _label)
  (`Widget.SetVisibility` _returnvalue "SelfHitTestInvisible" :!label _label_2)
  (bind _newparam (message `/Game/LiveToWin/Interfaces/BPI_WDamageValue.GetAnimation` _returnvalue))
  (`|PlayAnimation` _returnvalue _newparam 0.0 1 "Forward" 0.3
    (:`Finished`
      (`Widget.SetVisibility` _returnvalue "Collapsed"))))

(event `OnDamageTaken`
  (params (Damage :type Integer))
  (if (<= Damage 0)
    (goto _label)
    (else
      (message `/Game/LiveToWin/Interfaces/BPI_WDamageValue.SetDamageValue` (`WidgetComponent.GetWidget` (`self.Widget_Damage`)) Damage)
      (`/Game/LiveToWin/Components/BP_HealthComponent.DecreaseHealth` (`self.BP_HealthComponent`) Damage)
      (goto _label_2))))

(fn `Attack`
  (bind _returnvalue (`self.K2_GetActorLocation`))
  (bind _outhit (`KismetSystemLibrary.LineTraceSingle` :`Start` _returnvalue :`End` (+ _returnvalue (* (`self.GetActorForwardVector`) 3000.0)) :`TraceChannel` "TraceTypeQuery4" :`DrawDebugType` "ForDuration"))
  (bind (_bblockinghit _binitialoverlap _time _distance _location _impactpoint _normal _impactnormal _physmat _hitactor) (`GameplayStatics.BreakHitResult` _outhit))
  (if (`GameplayStatics.ObjectIsA` _hitactor "/Game/LiveToWin/Core/Characters/BP_BaseCharacter.BP_BaseCharacter_C")
    (bind _returnvalue_2 (`self.K2_GetActorLocation` _hitactor))
    (`AIBlueprintHelperLibrary.SimpleMoveToLocation` (`AIBlueprintHelperLibrary.GetAIController` self) _returnvalue_2)
    (set `self.PlayerLocation` _returnvalue_2)
    (bind _returnvalue_3 (`KismetSystemLibrary.K2_SetTimer` null "FindPlayer" 0.1 true))
    (set `self.FindPlayerTimerHandle` _returnvalue_3)))

(fn `CalculateFinalDamage`
  (params (BaseDamage :type "Float (double-precision)") (Attributes :type "/Game/LiveToWin/Components/F_Attributes Structure") (EnemyAttributes :type "/Game/LiveToWin/Components/F_Attributes Structure") (CauserWeaponInfo :type "/Game/LiveToWin/Weapons/F_WeaponInfo Structure"))
  (returns (FinalDamage :type Integer))
  (return 0))

(fn `EnableWeaponCollision`
  (`PrimitiveComponent.SetCollisionEnabled` (`/Game/LiveToWin/Weapons/BP_WeaponBase.DetectCapsule` (`self.Weapon`)) "QueryOnly"))

(fn `FindPlayer`
  (bind _returnvalue (`self.K2_GetActorLocation`))
  (bind _outhit (`KismetSystemLibrary.LineTraceSingle` :`Start` _returnvalue :`End` (+ _returnvalue (* (`self.GetActorForwardVector`) (`self.AttackRange`))) :`TraceChannel` "TraceTypeQuery4" :`DrawDebugType` "ForOneFrame"))
  (if (`GameplayStatics.ObjectIsA` (`.HitActor` (`GameplayStatics.BreakHitResult` _outhit)) "/Game/LiveToWin/Core/Characters/BP_BaseCharacter.BP_BaseCharacter_C")
    (`KismetSystemLibrary.K2_ClearAndInvalidateTimerHandle` (`self.FindPlayerTimerHandle`))
    (`MovementComponent.StopMovementImmediately` (`self.CharacterMovement`))
    (`self.MakeHit`)))

(fn `Get Weapon Type`
  (returns (WeaponType :type "/Game/LiveToWin/Weapons/E_Weapon Enum"))
  (return (`self.WeaponType`)))

(fn `GetAgility`
  (returns (AttAgility :type Integer))
  (return (`/Game/LiveToWin/Components/BP_AttributesComponent.Agility` (`self.BP_AttributesComponent`))))

(fn `GetAttributesStruct`
  (returns (Attributes :type "/Game/LiveToWin/Components/F_Attributes Structure"))
  (return (`/Game/LiveToWin/Components/BP_AttributesComponent.GetAttributesStruct` (`self.BP_AttributesComponent`))))

(fn `GetSpecialization`
  (returns (Specialization :type "Array of /Game/LiveToWin/Core/Characters/F_Specialization Structure"))
  (return))

(fn `GetWeaponInfo`
  (returns (WeaponInfo :type "/Game/LiveToWin/Weapons/F_WeaponInfo Structure"))
  (return (`/Game/LiveToWin/Weapons/BP_WeaponBase.WeaponInfo` (`self.Weapon`))))

(fn `IsAtStartLocation`
  (bind (_returnvalue_x _returnvalue_y) (`KismetMathLibrary.BreakVector` (`self.K2_GetActorLocation`)))
  (bind (_startlocation_x _startlocation_y) (`KismetMathLibrary.BreakVector` (`self.StartLocation`)))
  (if (and (`KismetMathLibrary.NearlyEqual_FloatFloat` _returnvalue_x _startlocation_x 1.0) (`KismetMathLibrary.NearlyEqual_FloatFloat` _returnvalue_y _startlocation_y 1.0))
    (`self.K2_SetActorRotation` (`KismetMathLibrary.FindLookAtRotation` (`self.K2_GetActorLocation`) (`self.PlayerLocation`)))
    (`KismetSystemLibrary.K2_ClearAndInvalidateTimerHandle` (`self.CheckStartLocationTimerHandle`))
    (`self.OnEnemyAttackEnded`)))

(fn `IsAttacking`
  (returns (Attacking :type Boolean))
  (return (`self.bAttacking`)))

(fn `MakeHit`
  (bind _attackanimations (`self.AttackAnimations`))
  (if (`KismetArrayLibrary.Array_IsNotEmpty` _attackanimations)
    (bind _returnvalue (`self.PlayAnimMontage` (`KismetArrayLibrary.Array_Random` _attackanimations)))
    (set `self.bAttacking` true)
    (`KismetSystemLibrary.K2_SetTimer` null "ReturnOnStartPosition" _returnvalue)
    (`KismetSystemLibrary.K2_SetTimer` null "EnableWeaponCollision" (* _returnvalue 0.35))))

(fn `ReturnOnStartPosition`
  (bind _startlocation (`self.StartLocation`))
  (set `self.bAttacking` false)
  (`self.K2_SetActorRotation` (`KismetMathLibrary.FindLookAtRotation` (`self.K2_GetActorLocation`) _startlocation))
  (`AIController.MoveToLocation` (`AIBlueprintHelperLibrary.GetAIController` self) _startlocation 1.0 false true false true null true)
  (bind _returnvalue (`KismetSystemLibrary.K2_SetTimer` null "IsAtStartLocation" 0.1 true))
  (set `self.CheckStartLocationTimerHandle` _returnvalue))

(fn `SpawnWeapon`
  (params (WeaponClass :type "/Game/LiveToWin/Weapons/BP_WeaponBase Class Reference"))
  (returns (SpawnedWeapon :type "/Game/LiveToWin/Weapons/BP_WeaponBase Object Reference"))
  (bind _returnvalue (`|SpawnActorFromClass` WeaponClass (`KismetMathLibrary.MakeTransform` (0.0 0.0 0.0)) "AlwaysSpawn" "MultiplyWithRoot" self null))
  (return _returnvalue))

(fn `UserConstructionScript`)