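; Golem character Blueprint that resolves incoming damage, deferring Tick and construction to its parent.
; On AnyDamage, it feeds the causer's and its own agility into a hit-rate check, triggering either a miss or damage taken.
; Its CalculateFinalDamage subtracts the golem's Stamina from truncated base damage, ignoring the attacker attributes and weapon info passed in.
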(event `self.ReceiveTick`
  (params (DeltaSeconds :type "Float (single-precision)"))
  (`parent.ReceiveTick` DeltaSeconds))

(event `self.ReceiveAnyDamage`
  (params (Damage :type "Float (single-precision)") (DamageType :type "DamageType Object Reference") (InstigatedBy :type "Controller Object Reference") (DamageCauser :type "Actor Object Reference"))
  (bind _attagility (message `/Game/LiveToWin/Interfaces/BPI_Battlable.GetAgility` DamageCauser))
  (bind _attagility_2 (`self.GetAgility`))
  (bind _miss (`/Game/LiveToWin/BFL_Battle.CalculateHitRate` _attagility _attagility_2))
  (if _miss
    (`self.OnAttackerMissed`)
    (else
      (bind _weaponinfo (message `/Game/LiveToWin/Interfaces/BPI_Battlable.GetWeaponInfo` DamageCauser))
      (bind _attributes (message `/Game/LiveToWin/Interfaces/BPI_Battlable.GetAttributesStruct` DamageCauser))
      (bind _finaldamage (`self.CalculateFinalDamage` Damage (`/Game/LiveToWin/Components/BP_AttributesComponent.GetAttributesStruct` (`self.BP_AttributesComponent`)) _attributes _weaponinfo))
      (`self.OnDamageTaken` _finaldamage))))

(fn `CalculateFinalDamage`
  (params (BaseDamage :type "Float (double-precision)") (Attributes :type "/Game/LiveToWin/Components/F_Attributes Structure") (EnemyAttributes :type "/Game/LiveToWin/Components/F_Attributes Structure") (CauserWeaponInfo :type "/Game/LiveToWin/Weapons/F_WeaponInfo Structure"))
  (returns (FinalDamage :type Integer))
  (return (- (`KismetMathLibrary.FTrunc` BaseDamage) (`.Stamina_8_8E07CCF048C5852763540F8C085369DE` (break `/Game/LiveToWin/Components/F_Attributes` Attributes)))))

(fn `UserConstructionScript`
  (`parent.UserConstructionScript`))