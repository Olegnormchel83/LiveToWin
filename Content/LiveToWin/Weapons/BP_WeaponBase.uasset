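; Base weapon Blueprint that applies melee damage to actors tagged Damagable when its detect capsule overlaps them while the owner is attacking.
; On a valid hit it disables the capsule's collision, and queries owner and target through message calls.
; A Ghost owner with higher agility than the target lands a hidden attack for one bonus damage.
; Helper functions expose weapon info, set damage, or raise it by Power.
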(event `self.ReceiveBeginPlay`
  (set `self.WeaponInfo` (make `/Game/LiveToWin/Weapons/F_WeaponInfo` (`self.Damage`) (`self.DamageType`))))

(event `self.DetectCapsule.OnComponentBeginOverlap`
  (params (OverlappedComponent :type "PrimitiveComponent Object Reference") (OtherActor :type "Actor Object Reference") (OtherComp :type "PrimitiveComponent Object Reference") (OtherBodyIndex :type Integer) (bFromSweep :type Boolean) (SweepResult :type "HitResult Structure (by ref)"))
  (bind _returnvalue (`self.GetOwner`))
  (bind _returnvalue_2 (`self.GetOwner`))
  (bind _attacking (message `/Game/LiveToWin/Interfaces/BPI_Battlable.IsAttacking` _returnvalue_2))
  (if (and _attacking (!= OtherActor _returnvalue_2) (`self.ActorHasTag` OtherActor "Damagable"))
    (`PrimitiveComponent.SetCollisionEnabled` (`self.DetectCapsule`) "NoCollision")
    ;[1 1 1] Проверка на Owner = Ghost
    (if (`GameplayStatics.ObjectIsA` _returnvalue "/Game/LiveToWin/Core/Characters/Ghost/BP_Ghost.BP_Ghost_C")
      (bind _attagility (message `/Game/LiveToWin/Interfaces/BPI_Battlable.GetAgility` _returnvalue))
      (bind _attagility_2 (message `/Game/LiveToWin/Interfaces/BPI_Battlable.GetAgility` OtherActor))
      (if (> _attagility _attagility_2)
        (`GameplayStatics.ApplyDamage` OtherActor (`KismetMathLibrary.Conv_IntToDouble` (+ (`self.Damage`) 1)))
        (`KismetSystemLibrary.PrintString` "Owner = Ghost, сработала \"Скрытая атака\"")
        (else
          (`GameplayStatics.ApplyDamage` OtherActor (`KismetMathLibrary.Conv_IntToDouble` (`self.Damage`)) :!label _label)))
      (else
        (goto _label)))))

(fn `AddDamageByPower`
  (params (Power :type Integer))
  (set `self.Damage` (+ (`self.Damage`) Power)))

(fn `GetWeaponInfo`
  (returns (Damage :type Integer) (DamageType :type "/Game/LiveToWin/Weapons/E_DamageType Enum"))
  (return (`self.Damage`) (`self.DamageType`)))

(fn `SetDamage`
  (params (Damage :type Integer))
  (set `self.Damage` Damage))

(fn `UserConstructionScript`)